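; Player paddle Blueprint for a Pong game that also owns the score HUD and reacts to a win.
; On BeginPlay it adds the Pong Enhanced Input mapping context and creates the score widget; the move action then slides the cube along Y with a swept offset.
; Tick polls the HUD's win flag to disable respawning on the ball and destroy it, while Escape calls the HUD's pause function.
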(event Input|EnhancedActionEvents|EnhancedInputActionMove_IA
  (params (ActionValue :type Float%20%28double-precision%29) (ElapsedSeconds :type Float%20%28double-precision%29) (TriggeredSeconds :type Float%20%28double-precision%29) (InputAction :type Input%20Action%20Object%20Reference :default "/Game/Input/Move_IA.Move_IA"))
  (Transformation|AddLocalOffset (Variables|Default|GetCube) (Math|Vector|MakeVector 0.0 (* ActionValue (Variables|Default|GetPlayerSpeed)) 0.0) true false))

(event EventBeginPlay
  (bind _asplayer_controller (Utilities|Casting|CastToPlayerController (Game|GetPlayerController 0)))
  (Utilities|IsValid (PlayerController|LocalPlayerSubsystems|GetEnhancedInputLocalPlayerSubsystem _asplayer_controller)
    (:Is%20Valid
      (Input|AddMappingContext (PlayerController|LocalPlayerSubsystems|GetEnhancedInputLocalPlayerSubsystem _asplayer_controller) "/Game/Input/Pong_IMC.Pong_IMC" 0 "(bIgnoreAllPressedKeysUntilRelease=True,bForceImmediately=False,bNotifyUserSettings=False)")
      (bind _returnvalue (UserInterface|CreateWidget "/Game/UI/Score_WBP.Score_WBP_C"))
      (bind _output_get (Variables|Default|SetScoreHUD _returnvalue))
      (UserInterface|Viewport|AddtoViewport _output_get 0))))

(event Collision|EventActorBeginOverlap
  (params (OtherActor :type Actor%20Object%20Reference)))

(event EventTick
  (params (DeltaSeconds :type Float%20%28single-precision%29))
  (if (Variables|/Game/UI/Score_WBP.Score_WBP_C|GetIsWon? (Variables|Default|GetScoreHUD))
    (bind _returnvalue (Actor|GetActorOfClass "/Game/Blueprints/Ball_BP.Ball_BP_C"))
    (Variables|Default|SetBallRef _returnvalue)
    (if (Utilities|IsValid (Variables|Default|GetBallRef))
      (Variables|/Game/Blueprints/Ball_BP.Ball_BP_C|SetShouldRespawn (Variables|Default|GetBallRef) false)
      (Actor|DestroyActor (Variables|Default|GetBallRef)))))

(event Input|KeyboardEvents|Escape
  (params (Key :type Key%20Structure :default "None"))
  (:Pressed
    (Default|GamePaused (Variables|Default|GetScoreHUD))))

(fn ConstructionScript)