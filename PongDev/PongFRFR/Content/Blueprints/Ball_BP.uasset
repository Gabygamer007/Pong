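; Pong ball actor that launches itself with a horizontal impulse, its side chosen by the Switch flag, plus a random sideways kick.
; On spawn it registers itself as BallRef on the AI_BP actor.
; Each hit plays a wall or paddle sound and raises the minimum speed, clamping physics velocity up to a fixed cap.
; When destroyed with ShouldRespawn set, it asks its spawner for a new ball.
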(event EventBeginPlay
  (Variables|Default|SetShouldRespawn true)
  (bind _returnvalue (Actor|GetActorOfClass "/Game/Blueprints/AI_BP.AI_BP_C"))
  (bind _output_get (Variables|Default|SetAI_Ref _returnvalue))
  (Variables|/Game/Blueprints/AI_BP.AI_BP_C|SetBallRef _output_get self)
  (if (Variables|Default|GetSwitch)
    (Physics|AddImpulse (Variables|Default|GetSphere) (Math|Vector|MakeVector 1e+03 (Math|Conversions|ToFloat(Integer) (Math|Random|RandomIntegerinRange -500 500)) 0.0) "None" true)
    (else
      (Physics|AddImpulse (Variables|Default|GetSphere) (Math|Vector|MakeVector -1e+03 (Math|Conversions|ToFloat(Integer) (Math|Random|RandomIntegerinRange -500 500)) 0.0) "None" true))))

(event Collision|EventActorBeginOverlap
  (params (OtherActor :type Actor%20Object%20Reference)))

(event EventTick
  (params (DeltaSeconds :type Float%20%28single-precision%29)))

(event Collision|EventHit
  (params (MyComp :type Primitive%20Component%20Object%20Reference) (Other :type Actor%20Object%20Reference) (OtherComp :type Primitive%20Component%20Object%20Reference) (bSelfMoved :type Boolean) (HitLocation :type Vector :default "0, 0, 0") (HitNormal :type Vector :default "0, 0, 0") (NormalImpulse :type Vector :default "0, 0, 0") (Hit :type Hit%20Result%20Structure%20%28by%20ref%29))
  (bind _sphere (Variables|Default|GetSphere))
  (if (Class|GameplayStatics|ObjectIsA Other "/Game/Blueprints/Wall_BP.Wall_BP_C")
    (Audio|PlaySoundatLocation "/Game/Sounds/PongHitWall.PongHitWall" "0, 0, 0" "0, 0, 0" 1.0 1.0 0.0 0 0 0 0)
    (else
      (Audio|PlaySoundatLocation "/Game/Sounds/PongHitPaddle.PongHitPaddle" "0, 0, 0" "0, 0, 0" 1.0 1.0 0.0 0 0 0 0)))
  (Variables|Default|SetBallspeed (+ (Variables|Default|GetBallspeed) 5e+01))
  (bind _returnvalue (Physics|GetPhysicsLinearVelocity _sphere "None"))
  (Physics|SetPhysicsLinearVelocity _sphere (Math|Vector|ClampVectorSize _returnvalue (Variables|Default|GetBallspeed) 2e+03) false "None"))

(event EventDestroyed
  (if (Variables|Default|GetShouldRespawn)
    (Default|SpawnBall (Variables|Default|GetBallSpawnerRef))))

(fn ConstructionScript)